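; BP_EnemyBase is an enemy character Blueprint that handles spawn-in, attack facing, death-style dissolves and loot drops.
; A timeline scales the mesh on BeginPlay, two others drive body and weapon material dissolves, and Motion Warping receives the facing target.
; SpawnLoot rolls items from loot tiers, then a looping timer spawns them one by one on evenly spaced rotations at random distances, optionally passing on the enemy's level.
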(event Custom|SpawnLootItem
  (bind _lootitems (Variables|Default|GetLootItems))
  (bind _spawnloopcount (Variables|Default|GetSpawnLoopCount))
  (bind _output (Utilities|Array|Get(acopy) _lootitems _spawnloopcount))
  (bind (_lootclass _blootleveloverride) (Utilities|Struct|BreakLootItem _output))
  (if (< (Variables|Default|GetSpawnLoopCount) (Utilities|Array|Length (Variables|Default|GetLootItems)))
    (bind _returnvalue (Game|SpawnActorfromClass _lootclass (CallFunction|GetLootTransform (Variables|Default|GetSpawnLoopCount)) "AlwaysSpawn" "MultiplyWithRoot" 0 0))
    (bind _asaura_effect_actor (Utilities|Casting|CastToAuraEffectActor _returnvalue)
      (:then
        (Utilities|IsValid _asaura_effect_actor
          (:Is%20Valid
            (if _blootleveloverride
              (Variables|/Script/GAS_Arua.AuraEffectActor|SetActorLevel _asaura_effect_actor (Math|Conversions|ToFloat(Integer) (Variables|Default|GetLevel)))))
          (:Is%20Not%20Valid
            _)))
      (:CastFailed
        _))
    (Math|Integer|IncrementInt (Variables|Default|GetSpawnLoopCount))
    (else
      (Utilities|Time|ClearandInvalidateTimerbyHandle (Variables|Default|GetLootTimer)))))

(event EventBeginPlay
  (bind _scaletrack (Timeline|SpawnTimeline Play)
    (:Update
      (Transformation|SetRelativeScale3D (Variables|Character|GetMesh) (Math|Vector|MakeVector _scaletrack _scaletrack _scaletrack)))))

(event Collision|EventActorBeginOverlap
  (params (OtherActor :type Actor%20Object%20Reference)))

(event EventTick
  (params (DeltaSeconds :type Float%20%28single-precision%29)))

(event EventStartDissolveTimeLine
  (params (DynamicMaterialInstance :type Material%20Instance%20Dynamic%20Object%20Reference))
  (bind _dissolvetrack (Timeline|Dissolve%20Timeline Play)
    (:Update
      (Rendering|Material|SetScalarParameterValue DynamicMaterialInstance "Dissolve" _dissolvetrack :!class /Script/Engine.MaterialInstanceDynamic))))

(event EventStartWeaponDissolveTimeLine
  (params (DynamicMaterialInstance :type Material%20Instance%20Dynamic%20Object%20Reference))
  (bind _dissolvetrack (Timeline|Weapon%20Dissolve%20Timeline Play)
    (:Update
      (Rendering|Material|SetScalarParameterValue DynamicMaterialInstance "Dissolve" _dissolvetrack :!class /Script/Engine.MaterialInstanceDynamic))))

(event EventUpdateFacingTarget
  (params (Target :type Vector%20%28by%20ref%29 :default "0, 0, 0"))
  (Class|MotionWarpingComponent|AddorUpdateWarpTargetfromLocation (Variables|Default|GetMotionWarping) "FacingTarget" Target))

(event EventSpawnLoot
  (bind _returnvalue (Class|AuraAbilitySystemLibrary|GetLootTiers))
  (bind _returnvalue_2 (Class|LootTiers|GetLootItems _returnvalue))
  (bind _output_get (Variables|Default|SetLootItems _returnvalue_2))
  (Variables|Default|SetLoot%20Rotations (CallFunction|GetLootRotaations _output_get))
  (Variables|Default|SetSpawnLoopCount 0)
  (bind _returnvalue_3 (Utilities|Time|SetTimerbyEvent (delegate Custom|SpawnLootItem) 0.1 true))
  (Variables|Default|SetLootTimer _returnvalue_3)
  (CallFunction|SpawnLootItem))

(fn ConstructionScript)

(fn GetLootRotaations
  (params (TargetArray :type Array%20of%20Loot%20Item%20Structures))
  (return (Class|AuraAbilitySystemLibrary|EvenlySpacedRotators (Transformation|GetActorForwardVector) (Math|Vector|VectorUp) 3.6e+02 (Utilities|Array|Length TargetArray))))

(fn GetLootTransform
  (params (LoopCount :type Integer))
  (bind _loot_rotations (Variables|Default|GetLoot%20Rotations))
  (bind _output (Utilities|Array|Get(acopy) _loot_rotations LoopCount))
  (return (Math|Transform|MakeTransform (+ (Transformation|GetActorLocation) (* (Math|Vector|GetForwardVector _output) (Math|Random|RandomFloatinRange (Variables|Default|GetMinSpawnDistance) (Variables|Default|GetMaxSpawnDistance_0)))) _output)))