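; Arcane Shards gameplay ability: shows a targeting magic circle, then erupts level-scaled, capped numbers of shards at the cursor.
; A second press or long-hold release spawns a randomly rotated BP_PointCollection for ground points and plays the cast montage.
; The montage event commits cost and starts a timer firing each shard's cue and radial damage, with pitched knockback from the cast center.
; Cooldown commits after the last shard, ending the ability.
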(event Custom|SetPoint
  (if (< (Variables|Default|GetCurrentNum) (Variables|Default|GetNumShards))
    (CallFunction|StoreShardsSpawnLocation)
    (CallFunction|StorePlayerstoDamage)
    (for _array_element (Variables|Default|GetPlayersToDamage)
      (CallFunction|ApplyRadialDamage _array_element))
    (Math|Integer|IncrementInt (Variables|Default|GetCurrentNum)
      (:%20%20
        (Class|GameplayAbility|ExecuteGameplayCuewithParams "(TagName=\"GameplayCue.ArcaneShards\")" (Ability|GameplayCue|MakeGameplayCueParameters :Location (Variables|Default|GetPointLocation)))))
    (else
      (Utilities|Time|ClearandInvalidateTimerbyHandle (Variables|Default|GetTimer))
      (Actor|DestroyActor (Variables|Default|GetPointCollection))
      (Ability|CommitAbilityCooldown false)
      (Ability|EndAbility))))

(event Ability|EventActivateAbility
  (bind _returnvalue (Class|GameplayAbility|CheckAbilityCost))
  (if _returnvalue
    (Utilities|FlowControl|Sequence
      (:then_0
        (Class|PlayerInterface|ShowMagicCircle(Message) (Ability|GetAvatarActorfromActorInfo) 0))
      (:then_1
        (Ability|Tasks|WaitInputPress false
          (:OnPress
            (bind _datahandle (|TargetDataUnderMouse :!label _label)
              (:ValidData
                (Variables|Default|SetMouseHitLocation (.ImpactPoint (Collision|BreakHitResult (Ability|TargetData|GetHitResultfromTargetData _datahandle))))
                (Utilities|FlowControl|Sequence
                  (:then_0
                    (bind _returnvalue_2 (Game|SpawnActorfromClass "/Game/BluePrints/AbilitySystem/Aura/Abilities/Arcane/ArcaneShards/BP_PointCollection.BP_PointCollection_C" (Math|Transform|MakeTransform (Variables|Default|GetMouseHitLocation) "0, 0, 0" "1.000000,1.000000,1.000000") "AlwaysSpawn" "MultiplyWithRoot" 0 0))
                    (Variables|Default|SetNumShards (Math|Integer|Min(Integer) (Variables|Default|GetMaxNumShards) (Ability|GetAbilityLevel)))
                    (Variables|Default|SetPointCollection _returnvalue_2)
                    (Variables|Default|SetArrayPoints (Class|PointCollection|GetGroundPoints (Variables|Default|GetPointCollection) (Variables|Default|GetMouseHitLocation) (Variables|Default|GetNumShards) (Math|Random|RandomFloatinRange 0.0 3.6e+02))))
                  (:then_1
                    (Class|CombatInterface|UpdateFacingTarget(Message) (Ability|GetAvatarActorfromActorInfo) (Variables|Default|GetMouseHitLocation)))
                  (:then_2
                    (|PlayMontageandWaitProxy "None" "/Game/Assets/Characters/Aura/Animations/Abilities/AM_Cast_ArcaneShards.AM_Cast_ArcaneShards" 1.0 "None" false 1.0 0.0 false
                      (:then
                        (Ability|Tasks|WaitGameplayEvent "(TagName=\"Event.Montage.ArcaneShards\")" 0 true
                          (:EventReceived
                            (bind _returnvalue_3 (Utilities|Time|SetTimerbyEvent (delegate Custom|SetPoint) (Variables|Default|GetSpawnShardsDeltaTime) true))
                            (Variables|Default|SetTimer _returnvalue_3)
                            (CallFunction|SetPoint)
                            (Class|PlayerInterface|HideMagicCircle(Message) (Ability|GetAvatarActorfromActorInfo))
                            (Ability|CommitAbilityCost false))))))))))))
      (:then_2
        (bind _timeheld (Ability|Tasks|WaitInputRelease false)
          (:OnRelease
            (if (>= _timeheld (Variables|Default|GetTriggerTIme))
              (goto _label))))))))

(event Ability|EventOnEndAbility
  (params (bWasCancelled :type Boolean))
  (Class|PlayerInterface|HideMagicCircle(Message) (Ability|GetAvatarActorfromActorInfo))
  (Utilities|Time|ClearandInvalidateTimerbyHandle (Variables|Default|GetTimer))
  (bind _pointcollection (Variables|Default|GetPointCollection)
    (:then
      (Actor|DestroyActor _pointcollection))
    (:else)))

(fn StoreShardsSpawnLocation
  (Variables|Default|SetPointLocation (Transformation|GetWorldLocation (Utilities|Array|Get(acopy) (Variables|Default|GetArrayPoints) (Variables|Default|GetCurrentNum))))
  (return))

(fn StorePlayerstoDamage
  (bind _returnvalue (Ability|GetAvatarActorfromActorInfo))
  (bind _outoverlappingactors (Class|AuraAbilitySystemLibrary|GetLivePlayerWithinRadius _returnvalue (Utilities|Array|MakeArray _returnvalue) (Variables|Default|GetRadialDamageOuterRadius) (Variables|Default|GetPointLocation)))
  (Variables|Default|SetPlayersToDamage _outoverlappingactors))

(fn ApplyRadialDamage
  (params (TargetActor :type Actor%20Object%20Reference))
  (bind _returnvalue (Transformation|GetActorLocation TargetActor))
  (bind _mousehitlocation (Variables|Default|GetMouseHitLocation))
  (bind _returnvalue_2 (- _returnvalue _mousehitlocation))
  (Class|AuraAbilitySystemLibrary|ApplyDamageEffect (Class|AuraDamageGameplayAbility|MakeDamageEffectParamfromClassDefault TargetActor (Variables|Default|GetMouseHitLocation) true _returnvalue_2 true _returnvalue_2 true 45.0)))