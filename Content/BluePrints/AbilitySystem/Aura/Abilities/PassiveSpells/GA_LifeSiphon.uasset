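; Passive Life Siphon gameplay ability that adjusts the owner's Health in proportion to incoming-damage events.
; On activation it waits for the Attributes.Meta.IncomingDamage gameplay event and multiplies the event magnitude by a level-based siphon magnitude.
; The result goes as a SetByCaller Health magnitude into a PassiveEffect spec at the ability's level, which is applied to the owner.
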(event Ability|EventActivateAbility
  (bind _returnvalue (Ability|GetAbilitySystemComponentfromActorInfo))
  (bind _payload (Ability|Tasks|WaitGameplayEvent "(TagName=\"Attributes.Meta.IncomingDamage\")" 0)
    (:EventReceived
      (bind _returnvalue_2 (Ability|GameplayEffect|AssignTagSetbyCallerMagnitude (GameplayEffects|MakeOutgoingSpec _returnvalue (Variables|Default|GetPassiveEffect) (Math|Conversions|ToFloat(Integer) (Ability|GetAbilityLevel)) (GameplayEffects|MakeEffectContext _returnvalue)) "(TagName=\"Attributes.Vital.Health\")" (* (Class|AuraLifeSiphon|GetSiphonMagnitude (Math|Conversions|ToFloat(Integer) (Ability|GetAbilityLevel))) (.EventMagnitude (Utilities|Struct|BreakGameplayEventData _payload)))))
      (Ability|ApplyGameplayEffectSpecToOwner _returnvalue_2))))

(event Ability|EventOnEndAbility
  (params (bWasCancelled :type Boolean)))